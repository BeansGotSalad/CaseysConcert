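; Park_light is a placeable park lamp Blueprint with a static mesh and a point light sharing one color and intensity.
; Its construction script applies LightColor and Intensity to the point light.
; It also creates a dynamic instance of an emissive material on the mesh's second slot, setting the same color and a tenth of the intensity so the glowing part matches the light.
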(fn ConstructionScript
  (Rendering|Components|Light|SetLightColor (Variables|Default|GetPointLight) (Variables|Default|GetlightColor) true)
  (bind _returnvalue (Rendering|Material|CreateDynamicMaterialInstance (Variables|Default|GetStaticMesh) 1 "/Game/Materials/Colors/Dynamic_emissive.Dynamic_emissive" "None" :!class /Script/Engine.PrimitiveComponent))
  (Rendering|Material|SetVectorParameterValue _returnvalue "Color" (Variables|Default|GetlightColor) :!class /Script/Engine.MaterialInstanceDynamic)
  (Rendering|Material|SetScalarParameterValue _returnvalue "Intensity" (/ (Variables|Default|Getintensity) 1e+01) :!class /Script/Engine.MaterialInstanceDynamic)
  (Rendering|Components|Light|SetIntensity (Variables|Default|GetPointLight) (Variables|Default|Getintensity)))