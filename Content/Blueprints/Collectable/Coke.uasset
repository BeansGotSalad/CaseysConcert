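; Collectable Coke pickup that increments the Coke count on the Casey character when it overlaps the sphere.
; A looping fast timer spins the paper sprite continuously around its yaw axis.
; On pickup it hides and disables sphere collision, then reappears after RespawnTime if that value is positive, otherwise staying hidden.
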(event OnComponentBeginOverlap(Sphere)
  (params (OverlappedComponent :type Primitive%20Component%20Object%20Reference) (OtherActor :type Actor%20Object%20Reference) (OtherComp :type Primitive%20Component%20Object%20Reference) (OtherBodyIndex :type Integer) (bFromSweep :type Boolean) (SweepResult :type Hit%20Result%20Structure%20%28by%20ref%29))
  ;[1 1 1] Overlap
  (bind _ascasey (Utilities|Casting|CastToCasey OtherActor))
  (Variables|/Game/Blueprints/Casey.Casey_C|Setcoke _ascasey (+ (Variables|/Game/Blueprints/Casey.Casey_C|Getcoke _ascasey) 1))
  (CallFunction|Hide))

(event Custom|SetCokeSpinTimer
  ;[1 1 1] Set coke spin timer
  (Utilities|Time|SetTimerbyFunctionName 0 "CokeSpin" 0.01 true))

(event Custom|CokeSpin
  ;[1 1 1] Coke spin
  (Transformation|AddWorldRotation (Variables|Default|GetPaperSprite) "0,1.000000, 0" false false))

(event Custom|Hide
  (Collision|SetCollisionEnabled (Variables|Default|GetSphere) "NoCollision")
  (Rendering|SetActorHiddenInGame true)
  (if (> (Variables|Default|GetrespawnTime) 0.0)
    (Utilities|Time|SetTimerbyFunctionName 0 "Unhide" (Variables|Default|GetrespawnTime))))

(event Custom|Unhide
  (Collision|SetCollisionEnabled (Variables|Default|GetSphere) "QueryOnly")
  (Rendering|SetActorHiddenInGame false))

(event EventBeginPlay
  ;[1 1 1] Begin play
  (CallFunction|SetCokeSpinTimer))

(fn ConstructionScript)