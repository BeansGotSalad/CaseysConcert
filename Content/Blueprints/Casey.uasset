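; Casey is the player character, with axis-driven movement and mouse look, jumping, a toggleable flashlight and a HUD created on BeginPlay.
; Tick polls Left Shift to switch walk speed between default and the current run speed.
; Left click spends a Coke charge to raise run speed briefly, with a looping one-second timer counting down, then restoring it and hiding the boost timer display.
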(event Custom|ShowCaseyHUD
  ;[1 1 1] Toggle Casey HUD
  (bind _returnvalue (UserInterface|CreateWidget "/Game/Blueprints/CaseyHUD.CaseyHUD_C"))
  (UserInterface|Viewport|AddtoViewport _returnvalue 0))

(event Custom|CokeSnort
  ;[1 1 1] Snort coke
  (if (> (Variables|Default|Getcoke) 0)
    (Variables|Default|Setcoke (- (Variables|Default|Getcoke) 1))
    (Utilities|Time|SetTimerbyFunctionName 0 "SpeedBoostTimerTick" 1.0 true)
    (Variables|Default|SetcurrentSpeedBoostTime 3.0)
    (Variables|Default|SetcurrentRunSpeed 2e+03)
    (Variables|Default|SetspeedBoostTImerVisibility "Visible")))

(event Custom|CheckForRun
  (bind _charactermovement (Variables|Character|GetCharacterMovement))
  ;[1 1 1] Run
  (if (Game|Player|IsInputKeyDown (Game|GetPlayerController 0) "LeftShift")
    (Variables|/Script/Engine.CharacterMovementComponent|SetMaxWalkSpeed _charactermovement (Variables|Default|GetcurrentRunSpeed)) ; Sprint speed
    (else
      (Variables|/Script/Engine.CharacterMovementComponent|SetMaxWalkSpeed _charactermovement (Variables|Default|GetdefaultWalkSpeed)) ; Default walk speed
    )))

(event Custom|SpeedBoostTimerTick
  ;[1 1 1] Speed boost timer tick
  (bind _output_get (Variables|Default|SetcurrentSpeedBoostTime (- (Variables|Default|GetcurrentSpeedBoostTime) 1.0)))
  (if (<= _output_get 0.0) ; Timer has ended
    (Variables|Default|SetcurrentRunSpeed (Variables|Default|GetdefaultRunSpeed))
    (Utilities|Time|ClearTimerbyFunctionName 0 "SpeedBoostTimerTick")
    (Variables|Default|SetspeedBoostTImerVisibility "Hidden")))

(event EventBeginPlay
  ;[1 1 1] Begin play
  (CallFunction|ShowCaseyHUD))

(event EventTick
  (params (DeltaSeconds :type Float%20%28single-precision%29))
  ;[1 1 1] Event tick
  (CallFunction|CheckforRun))

(event Input|ActionEvents|InputActionJump
  (params (Key :type Key%20Structure :default "None"))
  ;[1 1 1] Casey Jump
  (:Pressed
    (Character|Jump)))

(event Input|ActionEvents|InputActionFlashlight
  (params (Key :type Key%20Structure :default "None"))
  (bind _flashlight (Variables|Default|GetFlashlight))
  ;[1 1 1] Flashlight
  (:Pressed
    (if (Rendering|IsVisible _flashlight)
      (Rendering|SetVisibility _flashlight false false)
      (else
        (Rendering|SetVisibility _flashlight true false)))))

(event Input|AxisEvents|InputAxisforward_backward
  (params (AxisValue :type Float%20%28single-precision%29))
  ;[1 1 1] Casey Movement
  (Pawn|Input|AddMovementInput (Transformation|GetActorForwardVector) AxisValue false))

(event Input|AxisEvents|InputAxisstrafe_left_right
  (params (AxisValue :type Float%20%28single-precision%29))
  ;[1 1 1] Casey Movement
  (Pawn|Input|AddMovementInput (Transformation|GetActorRightVector) AxisValue false))

(event Input|AxisEvents|InputAxisrotate_left_right
  (params (AxisValue :type Float%20%28single-precision%29))
  ;[1 1 1] Mouse look
  (Pawn|Input|AddControllerYawInput AxisValue))

(event Input|AxisEvents|InputAxislook_up_down
  (params (AxisValue :type Float%20%28single-precision%29))
  ;[1 1 1] Mouse look
  (Pawn|Input|AddControllerPitchInput AxisValue))

(event Input|MouseEvents|LeftMouseButton
  (params (Key :type Key%20Structure :default "None"))
  ;[1 1 1] Coke snort input
  (:Pressed
    (CallFunction|CokeSnort)))

(fn ConstructionScript)